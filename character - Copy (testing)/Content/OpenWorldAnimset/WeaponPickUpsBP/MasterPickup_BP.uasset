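; Base weapon pickup actor that lets a ThirdPersonCharacter collect it through the ItemInteraction input.
; Sphere overlap toggles the prompt widget, the mesh's custom depth and a CanWePick flag, enabling input on entry.
; Pressing the input while in range passes the actor to the character's PickUp; OffAll hides the highlight and destroys the sphere.
; The construction script stamps the actor's own class into its ItemInfo struct.
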(event OnComponentBeginOverlap(Sphere)
  (params (OverlappedComponent :type Primitive%20Component%20Object%20Reference) (OtherActor :type Actor%20Object%20Reference) (OtherComp :type Primitive%20Component%20Object%20Reference) (OtherBodyIndex :type Integer) (bFromSweep :type Boolean) (SweepResult :type Hit%20Result%20Structure%20%28by%20ref%29))
  (bind _asthird_person_character (Utilities|Casting|CastToThirdPersonCharacter OtherActor))
  (Variables|Default|SetCharacterRef _asthird_person_character)
  (CallFunction|On/Off/Visibility/CustomDepth true true)
  (Variables|Default|SetCanWePick? true)
  (Input|EnableInput (Game|GetPlayerController 0)))

(event OnComponentEndOverlap(Sphere)
  (params (OverlappedComponent :type Primitive%20Component%20Object%20Reference) (OtherActor :type Actor%20Object%20Reference) (OtherComp :type Primitive%20Component%20Object%20Reference) (OtherBodyIndex :type Integer))
  (bind _asthird_person_character (Utilities|Casting|CastToThirdPersonCharacter OtherActor))
  (Variables|Default|SetCharacterRef _asthird_person_character)
  (CallFunction|On/Off/Visibility/CustomDepth false false)
  (Variables|Default|SetCanWePick? false))

(event Custom|OffAll
  (CallFunction|On/Off/Visibility/CustomDepth false false)
  (Components|DestroyComponent (Variables|Default|GetSphere))
  (Development|PrintString "Hello"))

(event Input|ActionEvents|InputActionItemInteraction
  (params (Key :type Key%20Structure))
  (:Pressed
    (if (Variables|Default|GetCanWePick?)
      (Default|PickUp (Variables|Default|GetCharacterRef) self))))

(fn ConstructionScript
  (Variables|Default|SetItemInfo (Utilities|Struct|MakeItemType (.itemtype (Variables|Default|GetItemInfo)) (Utilities|GetClass self) (.currentammo (Variables|Default|GetItemInfo)) (.maxammo (Variables|Default|GetItemInfo)) (.damage (Variables|Default|GetItemInfo)) (.itemimage (Variables|Default|GetItemInfo)) (.equipsocketname (Variables|Default|GetItemInfo)) (.unequipsocketname (Variables|Default|GetItemInfo)))))

(fn On/Off/Visibility/CustomDepth
  (params (bNewVisibility :type Boolean) (bValue :type Boolean))
  (Rendering|SetVisibility (Variables|Default|GetWidget) bNewVisibility false)
  (Rendering|SetRenderCustomDepth (Variables|Default|GetSkeletalMesh) bValue))