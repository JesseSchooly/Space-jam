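; Base weapon actor that assembles a configurable gun's appearance from a paint mode and attachment choices; it has no firing or gameplay logic.
; The Construction Script snaps the magazine to its socket, then runs functions for paint, grip, barrel and scope.
; Paint uses a base material or a dynamic instance for color or skin texture.
; Attachment functions swap meshes on named sockets, skipping certain weapon types; grip and barrel can also be hidden.
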(event EventBeginPlay)

(event Collision|EventActorBeginOverlap
  (params (OtherActor :type Actor%20Object%20Reference)))

(event EventTick
  (params (DeltaSeconds :type Float%20%28single-precision%29)))

(fn ConstructionScript
  (Transformation|AttachComponentToComponent (Variables|Default|GetMag) (Variables|Default|GetWeapon_Mesh) "Mag" "SnapToTarget" "SnapToTarget" "SnapToTarget" false)
  (CallFunction|SetPaintMode)
  (CallFunction|SetGrip)
  (CallFunction|SetBarrel)
  (CallFunction|SetScope))

(fn SetPaintMode
  (bind _weapon_mesh (Variables|Default|GetWeapon_Mesh))
  (bind _weapon_mesh_2 (Variables|Default|GetWeapon_Mesh))
  (if (Utilities|Enum|Equal(Enum) (Variables|Modification|GetPaintMode:) "NewEnumerator0")
    (Rendering|Material|SetMaterial (Variables|Default|GetWeapon_Mesh) 0 (Variables|Paint|GetBaseColor_mat))
    (elif (Utilities|Enum|Equal(Enum) (Variables|Modification|GetPaintMode:) "NewEnumerator1")
      (bind _returnvalue (Rendering|Material|CreateDynamicMaterialInstance _weapon_mesh 0 (Variables|Paint|GetColor_Mat) :!class /Script/Engine.PrimitiveComponent))
      (bind _output_get (Variables|Paint|SetColor_Inst _returnvalue))
      (Rendering|Material|SetMaterial _weapon_mesh 0 _output_get)
      (Rendering|Material|SetVectorParameterValue (Variables|Paint|GetColor_Inst) "SkinColor" (Variables|Modification|GetColor%20:) :!class /Script/Engine.MaterialInstanceDynamic)
      (elif (Utilities|Enum|Equal(Enum) (Variables|Modification|GetPaintMode:) "NewEnumerator2")
        (bind _returnvalue_2 (Rendering|Material|CreateDynamicMaterialInstance _weapon_mesh_2 0 (Variables|Paint|GetSkin_Mat) :!class /Script/Engine.PrimitiveComponent))
        (bind _output_get_2 (Variables|Paint|SetSkin_Inst _returnvalue_2))
        (Rendering|Material|SetMaterial _weapon_mesh_2 0 _output_get_2)
        (Rendering|Material|SetTextureParameterValue (Variables|Paint|GetSkin_Inst) "SkinTexture" (Variables|Modification|GetSkin%20Texture%20:))
        (Rendering|Material|SetScalarParameterValue (Variables|Paint|GetSkin_Inst) "Texture_Scale" (Variables|Modification|GetTexture%20UV%20Scale%20:) :!class /Script/Engine.MaterialInstanceDynamic)))))

(fn SetGrip
  (if (not (or (Utilities|Enum|Equal(Enum) (Variables|Default|GetWeaponType) "NewEnumerator0") (Utilities|Enum|Equal(Enum) (Variables|Default|GetWeaponType) "NewEnumerator4")))
    (if (Utilities|Enum|Equal(Enum) (Variables|Modification|GetFore%20Grip:) "NewEnumerator3")
      (Rendering|SetVisibility (Variables|Default|GetGrip) false false)
      (elif (Utilities|Enum|Equal(Enum) (Variables|Modification|GetFore%20Grip:) "NewEnumerator0")
        (Components|StaticMesh|SetStaticMesh (Variables|Default|GetGrip) "/Game/Weapons/Mesh/Attachment/SM_VerticleTypeA_Grip.SM_VerticleTypeA_Grip")
        (Transformation|AttachComponentToComponent (Variables|Default|GetGrip) (Variables|Default|GetWeapon_Mesh) (Variables|Grip|GetGrip_Socket) "SnapToTarget" "SnapToTarget" "SnapToTarget" false)
        (elif (Utilities|Enum|Equal(Enum) (Variables|Modification|GetFore%20Grip:) "NewEnumerator1")
          (Components|StaticMesh|SetStaticMesh (Variables|Default|GetGrip) "/Game/Weapons/Mesh/Attachment/SM_VerticleTypeB_Grip.SM_VerticleTypeB_Grip")
          (Transformation|AttachComponentToComponent (Variables|Default|GetGrip) (Variables|Default|GetWeapon_Mesh) (Variables|Grip|GetGrip_Socket) "SnapToTarget" "SnapToTarget" "SnapToTarget" false)
          (elif (Utilities|Enum|Equal(Enum) (Variables|Modification|GetFore%20Grip:) "NewEnumerator2")
            (Components|StaticMesh|SetStaticMesh (Variables|Default|GetGrip) "/Game/Weapons/Mesh/Attachment/SM_Angled_Grip.SM_Angled_Grip")
            (Transformation|AttachComponentToComponent (Variables|Default|GetGrip) (Variables|Default|GetWeapon_Mesh) (Variables|Grip|GetGripAngle_Socket) "SnapToTarget" "SnapToTarget" "SnapToTarget" false)))))))

(fn SetBarrel
  (if (not (Utilities|Enum|Equal(Enum) (Variables|Default|GetWeaponType) "NewEnumerator4"))
    (if (Utilities|Enum|Equal(Enum) (Variables|Modification|GetBarrel%20Type:) "NewEnumerator4")
      (Rendering|SetVisibility (Variables|Default|GetBarrel) false false)
      (elif (Utilities|Enum|Equal(Enum) (Variables|Modification|GetBarrel%20Type:) "NewEnumerator1")
        (Components|StaticMesh|SetStaticMesh (Variables|Default|GetBarrel) "/Game/Weapons/Mesh/Attachment/SM_MuzzleBrake_Barrel.SM_MuzzleBrake_Barrel")
        (Transformation|AttachComponentToComponent (Variables|Default|GetBarrel) (Variables|Default|GetWeapon_Mesh) (Variables|Barrel|GetBarrel_socket) "SnapToTarget" "SnapToTarget" "SnapToTarget" false)
        (elif (Utilities|Enum|Equal(Enum) (Variables|Modification|GetBarrel%20Type:) "NewEnumerator2")
          (Components|StaticMesh|SetStaticMesh (Variables|Default|GetBarrel) "/Game/Weapons/Mesh/Attachment/SM_FlashHidder_Barrel.SM_FlashHidder_Barrel")
          (Transformation|AttachComponentToComponent (Variables|Default|GetBarrel) (Variables|Default|GetWeapon_Mesh) (Variables|Barrel|GetBarrel_socket) "SnapToTarget" "SnapToTarget" "SnapToTarget" false)
          (elif (Utilities|Enum|Equal(Enum) (Variables|Modification|GetBarrel%20Type:) "NewEnumerator3")
            (Components|StaticMesh|SetStaticMesh (Variables|Default|GetBarrel) "/Game/Weapons/Mesh/Attachment/SM_Silencer_Barrel.SM_Silencer_Barrel")
            (Transformation|AttachComponentToComponent (Variables|Default|GetBarrel) (Variables|Default|GetWeapon_Mesh) (Variables|Barrel|GetBarrel_socket) "SnapToTarget" "SnapToTarget" "SnapToTarget" false)))))))

(fn SetScope
  (if (not (Utilities|Enum|Equal(Enum) (Variables|Default|GetWeaponType) "NewEnumerator4"))
    (if (Utilities|Enum|Equal(Enum) (Variables|Modification|GetScope%20Type:) "NewEnumerator1")
      (Components|StaticMesh|SetStaticMesh (Variables|Default|GetScope) (Variables|Scope|GetIronSight))
      (Transformation|AttachComponentToComponent (Variables|Default|GetScope) (Variables|Default|GetWeapon_Mesh) (Variables|Scope|GetIronSightSocket) "SnapToTarget" "SnapToTarget" "SnapToTarget" false)
      (elif (Utilities|Enum|Equal(Enum) (Variables|Modification|GetScope%20Type:) "NewEnumerator2")
        (Components|StaticMesh|SetStaticMesh (Variables|Default|GetScope) "/Game/Weapons/Mesh/Attachment/SM_RedDotSight_Scope.SM_RedDotSight_Scope")
        (Transformation|AttachComponentToComponent (Variables|Default|GetScope) (Variables|Default|GetWeapon_Mesh) (Variables|Scope|GetScopeSocket) "SnapToTarget" "SnapToTarget" "SnapToTarget" false)
        (elif (Utilities|Enum|Equal(Enum) (Variables|Modification|GetScope%20Type:) "NewEnumerator3")
          (Components|StaticMesh|SetStaticMesh (Variables|Default|GetScope) "/Game/Weapons/Mesh/Attachment/SM_Holographic_Scope.SM_Holographic_Scope")
          (Transformation|AttachComponentToComponent (Variables|Default|GetScope) (Variables|Default|GetWeapon_Mesh) (Variables|Scope|GetScopeSocket) "SnapToTarget" "SnapToTarget" "SnapToTarget" false)
          (elif (Utilities|Enum|Equal(Enum) (Variables|Modification|GetScope%20Type:) "NewEnumerator4")
            (Components|StaticMesh|SetStaticMesh (Variables|Default|GetScope) "/Game/Weapons/Mesh/Attachment/SM_ACOG_Scope.SM_ACOG_Scope")
            (Transformation|AttachComponentToComponent (Variables|Default|GetScope) (Variables|Default|GetWeapon_Mesh) (Variables|Scope|GetScopeSocket) "SnapToTarget" "SnapToTarget" "SnapToTarget" false)))))))